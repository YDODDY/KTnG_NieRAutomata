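; Boss character that chases the first player and pauses for two seconds when flagged as attacked.
; Every Tick runs FollowPlayer, which sets walking mode and issues AIMoveTo toward the player, with debug prints.
; When IsAttacked is true, it disables movement, waits, then clears the flag, sets movement mode None and reissues the move.
; Nothing in these graphs sets IsAttacked to true.
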(event Custom|FollowPlayer
  (if (Variables|Default|GetIsAttacked?)
    ;[1 1 1] 맞으면 2초 멈췄다가 다시 따라옴
    (Pawn|Components|CharacterMovement|DisableMovement (Variables|Character|GetCharacterMovement))
    (Development|PrintString "Attacked")
    (Utilities|FlowControl|Delay 2.0)
    (Variables|Default|SetIsAttacked? false)
    (Pawn|Components|CharacterMovement|SetMovementMode (Variables|Character|GetCharacterMovement) "MOVE_None" 0)
    (else
      ;[1 1 1] Player 따라옴
      (Pawn|Components|CharacterMovement|SetMovementMode (Variables|Character|GetCharacterMovement) "MOVE_Walking" 0)))
  (Development|PrintString "Follow Player")
  (AI|AIMoveTo self "0, 0, 0" (Game|GetPlayerCharacter 0) 5.0 false))

(event Collision|EventActorBeginOverlap
  (params (OtherActor :type Actor%20Object%20Reference)))

(event EventTick
  (params (DeltaSeconds :type Float%20%28single-precision%29))
  (CallFunction|FollowPlayer))

(fn ConstructionScript)